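; BP_Player is the Paper2D-style player character with flipbook run, jump, attack and death, health regen, and soul-based leveling.
; Enhanced Input drives movement and jumping, with a delay loop polling Z velocity for landing.
; The Z key starts an attack; Tick fires a DoOnce-gated hitbox overlap damage check at flipbook frame 3, re-armed when playback finishes.
; BeginPlay adds the UI and starts recursive regen; U and F are debug keys.
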(event `Reset Attack`
  (goto _label :!via `Reset`))

(event `self.ReceiveTick`
  (params (DeltaSeconds :type "Float (single-precision)"))
  (if (`self.isAttacking`)
    (if (== (`PaperFlipbookComponent.GetPlaybackPositionInFrames` (`self.Sprite`)) 3)
      (`/Engine/EditorBlueprintResources/StandardMacros.DoOnce` false :!label _label
        (:`Completed`
          (`self.HitCheck`))))))

(event `self.ReceiveBeginPlay`
  ;[1 1 1] keymapping
  (bind _returnvalue (`|CreateWidget` "/Game/Blueprints/UI/PlayerUI.PlayerUI_C" (`GameplayStatics.GetPlayerController` 0)))
  (`UserWidget.AddToViewport` _returnvalue 0)
  (bind _asbp_player_controller (cast `/Game/Blueprints/BP_PlayerController` (`self.GetController`)))
  (`EnhancedInputSubsystemInterface.AddMappingContext` (pcsubsystem `EnhancedInputLocalPlayerSubsystem` _asbp_player_controller) "/Game/Blueprints/IMC_Default.IMC_Default" 0 (struct))
  (`self.PassiveHPRegen`))

(event `EnhancedInput|/Game/Blueprints/IA_Movement`
  (params (ActionValue :type "Float (double-precision)") (ElapsedSeconds :type "Float (double-precision)") (TriggeredSeconds :type "Float (double-precision)") (InputAction :type "InputAction Object Reference" :default "/Game/Blueprints/IA_Movement.IA_Movement"))
  (bind _returnvalue (* ActionValue (`self.MovementSpeed`)))
  (:`Triggered`
    ;[1 1 1] Movement
    (if (`self.isDead`)
      _
      (elif (not (`self.isJumping`))
        (`self.AddMovementInput` (`self.GetActorForwardVector`) _returnvalue)
        (`PaperFlipbookComponent.SetFlipbook` (`self.Sprite`) "/Game/Assets/FinalStuffs/PlayerFlipbooks/FB_Run.FB_Run")
        (if (> _returnvalue 0.0)
          (`SceneComponent.K2_SetWorldRotation` :`self` (`self.Sprite`))
          (else
            (`SceneComponent.K2_SetWorldRotation` (`self.Sprite`) (struct :`Yaw` -180.0) false false))))))
  (:`Completed`
    (if (`self.isDead`)
      _
      (elif (not (`self.isJumping`))
        (`PaperFlipbookComponent.SetFlipbook` (`self.Sprite`) "/Game/Assets/FinalStuffs/PlayerFlipbooks/FB_Idle.FB_Idle")))))

(event `EnhancedInput|/Game/Blueprints/IA_Jump`
  (params (ActionValue :type Boolean) (ElapsedSeconds :type "Float (double-precision)") (TriggeredSeconds :type "Float (double-precision)") (InputAction :type "InputAction Object Reference" :default "/Game/Blueprints/IA_Jump.IA_Jump"))
  (bind (_returnvalue_x _returnvalue_y _returnvalue_z) (`KismetMathLibrary.BreakVector` (`self.GetVelocity`)))
  (bind _sprite (`self.Sprite`))
  ;[1 1 1] Jumping
  (:`Triggered`
    (if (`self.isDead`)
      _
      (elif (not (`self.isJumping`))
        (set `self.isJumping` true)
        (`self.Jump`)
        (`PaperFlipbookComponent.SetLooping` _sprite false)
        (`PaperFlipbookComponent.SetFlipbook` _sprite "/Game/Assets/FinalStuffs/PlayerFlipbooks/FB_Jump.FB_Jump")
        (`KismetSystemLibrary.Delay` 0.1)
        (if (== _returnvalue_z 0.0) :!label _label_2
          (`PaperFlipbookComponent.SetLooping` _sprite true)
          (`PaperFlipbookComponent.Play` _sprite)
          (`PaperFlipbookComponent.SetFlipbook` _sprite "/Game/Assets/FinalStuffs/PlayerFlipbooks/FB_Idle.FB_Idle")
          (set `self.isJumping` false)
          (else
            (`KismetSystemLibrary.Delay` 0.1)
            (goto _label_2)))))))

(event `AddSouls`
  (params (Increment :type Integer))
  ;[1 1 1] Exp system
  (set `self.Souls` (+ (`self.Souls`) Increment))
  (if (>= (`self.Souls`) (`self.MaxSouls`))
    (set `self.Souls` (- (`self.Souls`) (`self.MaxSouls`)))
    (`/Engine/EditorBlueprintResources/StandardMacros.IncrementInt` (`self.Level`)
      (:`  `
        (`/Engine/EditorBlueprintResources/StandardMacros.IncrementInt` (`self.SoulPoints`)
          (:`  `
            (set `self.MaxSouls` (`KismetMathLibrary.FTrunc` (+ (`KismetMathLibrary.MultiplyMultiply_FloatFloat` (/ (`self.Level`) 0.3) 2.0) 100.0)))))))))

(event `PassiveHPRegen`
  ;[1 1 1] Passive HP regen
  (if (`self.isDead`)
    _
    (elif (< (`self.CurrentHealth`) (`self.MaxHealth`))
      (set `self.CurrentHealth` (+ (`self.CurrentHealth`) (`self.RegenHP`)))
      (`KismetSystemLibrary.Delay` 1.0)
      (`self.PassiveHPRegen`)
      (else
        (`KismetSystemLibrary.Delay` 1.0)
        (`self.PassiveHPRegen`)))))

(event `self.ReceiveAnyDamage`
  (params (Damage :type "Float (single-precision)") (DamageType :type "DamageType Object Reference") (InstigatedBy :type "Controller Object Reference") (DamageCauser :type "Actor Object Reference"))
  (bind _sprite (`self.Sprite`))
  ;[1 1 1] Character taking damage
  (set `self.CurrentHealth` (`KismetMathLibrary.Clamp` (- (`self.CurrentHealth`) Damage) 0 (`self.MaxHealth`)))
  (if (== (`self.CurrentHealth`) 0)
    (set `self.isDead` true)
    (`PaperFlipbookComponent.SetFlipbook` _sprite "/Game/Assets/FinalStuffs/PlayerFlipbooks/Death_FB.Death_FB")
    (`PaperFlipbookComponent.SetLooping` _sprite false)))

(event `Key|U`
  (params (Key :type "Key Structure"))
  ;[1 1 1] Character taking damage
  (:`Pressed`
    (set `self.CurrentHealth` 0)))

(event `Key|F`
  (params (Key :type "Key Structure"))
  ;[1 1 1] Dev testing exp system
  (:`Pressed`
    (`self.AddSouls` 30)
    (`KismetSystemLibrary.PrintString` (`KismetStringLibrary.Concat_StrStr` "Souls: " (`KismetStringLibrary.Conv_IntToString` (`self.Souls`))))
    (`KismetSystemLibrary.PrintString` (`KismetStringLibrary.Concat_StrStr` "Max Souls: " (`KismetStringLibrary.Conv_IntToString` (`self.MaxSouls`))))
    (`KismetSystemLibrary.PrintString` (`KismetStringLibrary.Concat_StrStr` "Level: " (`KismetStringLibrary.Conv_IntToString` (`self.Level`))))))

(event `Key|X`
  (params (Key :type "Key Structure")))

(event `Key|Z`
  (params (Key :type "Key Structure"))
  (:`Pressed`
    (`PaperFlipbookComponent.SetFlipbook` (`self.Sprite`) "/Game/Assets/FinalStuffs/PlayerFlipbooks/FB_Attack.FB_Attack")
    (`PaperFlipbookComponent.SetLooping` (`self.Sprite`) false)
    (set `self.isAttacking` true)
    (`SceneComponent.SetHiddenInGame` (`self.AttackHitbox`) false false)))

(event `self.Sprite.OnFinishedPlaying`
  (if (not (`self.isDead`))
    (`PaperFlipbookComponent.SetFlipbook` (`self.Sprite`) "/Game/Assets/FinalStuffs/PlayerFlipbooks/FB_Idle.FB_Idle")
    (`self.Restart animation`)
    (set `self.isAttacking` false)
    (`SceneComponent.SetHiddenInGame` (`self.AttackHitbox`) true false)
    (`self.Reset Attack`)))

(fn `HitCheck`
  (for _array_element (`PrimitiveComponent.GetOverlappingActors` (`self.AttackHitbox`) null)
    (if (!= _array_element self)
      (`GameplayStatics.ApplyDamage` _array_element (`self.Damage Amount`) null self))))

(fn `Restart animation`
  (`PaperFlipbookComponent.SetLooping` (`self.Sprite`) true)
  (if (not (`PaperFlipbookComponent.IsPlaying` (`self.Sprite`)))
    (`PaperFlipbookComponent.Play` (`self.Sprite`))))

(fn `UserConstructionScript`)