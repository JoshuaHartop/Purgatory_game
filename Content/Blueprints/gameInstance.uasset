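; Game instance that manages a cooldown for teleporting to the hub level.
; HubTP opens Level_Hub only when HubCD exactly equals 600, then resets it to zero and starts HubTeleportCD.
; HubTeleportCD delays by HubCD seconds, increments it and calls itself.
; Its limit check compares constant zero to 600, so the loop never stops and each wait grows with the counter.
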(event `HubTeleportCD`
  (`KismetSystemLibrary.Delay` (`self.hubCD`))
  (if (< 0.0 600.0)
    (`/Engine/EditorBlueprintResources/StandardMacros.IncrementFloat` (`self.hubCD`)
      (:`  `
        (`self.HubTeleportCD`)))))

(event `HubTP`
  (if (== (`self.hubCD`) 600.0)
    (`GameplayStatics.OpenLevelBySoftObjectPtr` "/Game/Maps/Level_Hub.Level_Hub")
    (set `self.hubCD` 0.0)
    (`self.HubTeleportCD`)))