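; BP_FloatingTextActor is a short-lived actor that displays floating combat text through a widget component.
; Initialize stores the text, and BeginPlay passes it to the FloatingCombatTextWidget's Init after binding to that widget's animation-finish event.
; The actor destroys itself when the animation finishes.
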(event `self.ReceiveBeginPlay`
  (bind _asfloating_combat_text_widget (cast `/Game/Assets/FinalStuffs/FloatingCombatText/FloatingCombatTextWidget` (`WidgetComponent.GetUserWidgetObject` (`self.Widget`))))
  (add `/Game/Assets/FinalStuffs/FloatingCombatText/FloatingCombatTextWidget.AnimationFinish` _asfloating_combat_text_widget (`|CreateDelegate` :!event `HandleAnimationFinish`))
  (`/Game/Assets/FinalStuffs/FloatingCombatText/FloatingCombatTextWidget.Init` _asfloating_combat_text_widget (`self.Text`)))

(event `self.Initialize`
  (params (text :type "Text (by ref)"))
  (set `self.Text` text))

(fn `HandleAnimationFinish`
  ;[1 1 1] Destroy actor when animation is finished
  (`self.K2_DestroyActor`))

(fn `UserConstructionScript`)